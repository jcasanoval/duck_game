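; BP_Duckling is a duckling character that joins a follow chain when a BP_ThirdPersonCharacter overlaps its capsule.
; On first overlap it follows that character's LastDuckling, then registers itself as the new LastDuckling.
; FollowPlayer4 re-issues AI MoveTo toward the target's current location after each success or failure, teleporting to an offset near the target when a move fails far away.
; The FollowPlayer function is empty.
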(event OnComponentBeginOverlap(CapsuleComponent)
  (params (OverlappedComponent :type Primitive%20Component%20Object%20Reference) (OtherActor :type Actor%20Object%20Reference) (OtherComp :type Primitive%20Component%20Object%20Reference) (OtherBodyIndex :type Integer) (bFromSweep :type Boolean) (SweepResult :type Hit%20Result%20Structure%20%28by%20ref%29))
  (if (not (Variables|Default|GetFollowing))
    (bind _asbp_third_person_character (Utilities|Casting|CastToBP_ThirdPersonCharacter OtherActor))
    (CallFunction|FollowPlayer4 (Variables|/Game/ThirdPerson/Blueprints/BP_ThirdPersonCharacter.BP_ThirdPersonCharacter_C|GetLastDuckling _asbp_third_person_character))
    (Variables|/Game/ThirdPerson/Blueprints/BP_ThirdPersonCharacter.BP_ThirdPersonCharacter_C|SetLastDuckling _asbp_third_person_character self)
    (Variables|Default|SetFollowing true)))

(event Custom|Follow%20Player4
  (params (Follow :type Pawn%20Object%20Reference%20%28by%20ref%29))
  (AI|AIMoveTo self (.location (Transformation|GetActorTransform Follow)) 0 2e+02 false
    (:OnSuccess
      _)
    (:OnFail
      (if (>= (Transformation|GetDistanceTo Follow) 1e+03)
        (Transformation|SetActorLocation (+ (Transformation|GetActorLocation Follow) "500.000000,500.000000,20.000000") false false))))
  (CallFunction|FollowPlayer4 Follow))

(event EventBeginPlay
  (Variables|Default|SetFollowing false))

(fn ConstructionScript)

(fn FollowPlayer
  (params (Follow1 :type Pawn%20Object%20Reference%20%28by%20ref%29)))