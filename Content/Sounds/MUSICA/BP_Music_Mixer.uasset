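; BP_Music_Mixer builds layered adaptive music that follows how many ducklings are following.
; Every Tick it finds all BP_Duckling actors and counts those with Following set.
; That count, from one to ten, selects one instrument layer and sets its volume multiplier to full.
; Only the layer matching the exact count is touched, and nothing here lowers a layer when the count drops.
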(event EventTick
  (params (DeltaSeconds :type Float%20%28single-precision%29))
  (bind _outactors (Actor|GetAllActorsOfClass "/Game/Characters/BP_Duckling.BP_Duckling_C"))
  (Variables|Default|SetFoundDucks 0)
  (for _array_element _outactors
    (if (Variables|/Game/Characters/BP_Duckling.BP_Duckling_C|GetFollowing _array_element)
      (Math|Integer|IncrementInt (Variables|Default|GetFoundDucks))))
  (switch int (Variables|Default|GetFoundDucks)
    (:1
      (Audio|Components|Audio|SetVolumeMultiplier (Variables|Default|GetCAPA_1_PAD) 1.0 :!class /Script/Engine.AudioComponent))
    (:2
      (Audio|Components|Audio|SetVolumeMultiplier (Variables|Default|GetCAPA_2BELL) 1.0 :!class /Script/Engine.AudioComponent))
    (:3
      (Audio|Components|Audio|SetVolumeMultiplier (Variables|Default|GetCAPA_3_PNO_UP) 1.0 :!class /Script/Engine.AudioComponent))
    (:4
      (Audio|Components|Audio|SetVolumeMultiplier (Variables|Default|GetCAPA_4_RISE) 1.0 :!class /Script/Engine.AudioComponent))
    (:5
      (Audio|Components|Audio|SetVolumeMultiplier (Variables|Default|GetCAPA_5_BRASS) 1.0 :!class /Script/Engine.AudioComponent))
    (:6
      (Audio|Components|Audio|SetVolumeMultiplier (Variables|Default|GetCAPA_6_PNo) 1.0 :!class /Script/Engine.AudioComponent))
    (:7
      (Audio|Components|Audio|SetVolumeMultiplier (Variables|Default|GetCAPA_7_GT) 1.0 :!class /Script/Engine.AudioComponent))
    (:8
      (Audio|Components|Audio|SetVolumeMultiplier (Variables|Default|GetCAPA_8_AC) 1.0 :!class /Script/Engine.AudioComponent))
    (:9
      (Audio|Components|Audio|SetVolumeMultiplier (Variables|Default|GetCAPA_9_STAC) 1.0 :!class /Script/Engine.AudioComponent))
    (:10
      (Audio|Components|Audio|SetVolumeMultiplier (Variables|Default|GetCAPA_10_ARPS) 1.0 :!class /Script/Engine.AudioComponent))))

(fn ConstructionScript)